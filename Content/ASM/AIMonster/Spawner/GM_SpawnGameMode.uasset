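; Game mode that runs server-side monster waves, spawning goblins, kobolds and trolls at random BP_SpawnPoint actors.
; PopulateMap loads each wave's per-type counts from DT_WaveDetails into a map and total.
; A looping timer spawns through ChooseEnemy, which rerolls until it finds a type with remaining count.
; When no monsters remain, it delays the next wave and prints Clear, Ready or Finish; the UI widget code is disconnected.
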(event Custom|ActivateSpawner
  (bind _spawnlist (Variables|Default|GetSpawnList))
  (Networking|SwitchHasAuthority
    (:Authority
      (if (> (Variables|Default|GetNumberOfEnemies) 0)
        (bind _enemychosen (CallFunction|ChooseEnemy))
        (Default|SpawnEnemy (Utilities|Array|Get(acopy) _spawnlist (Math|Random|RandomIntegerinRange 0 (- (Utilities|Array|Length _spawnlist) 1))) _enemychosen)
        (else
          (bind _outactors (Actor|GetAllActorsOfClass "/Game/ASM/AIMonster/Monsters/BP_MasterMonster.BP_MasterMonster_C"))
          (if (<= (Utilities|Array|Length _outactors) 0)
            (Utilities|FlowControl|Sequence
              (:then_0
                (Networking|SwitchHasAuthority
                  (:Authority
                    (Utilities|FlowControl|Delay 2e+01)
                    (bind _result (Math|Integer|IncrementInt (Variables|Default|GetWaveNumber))
                      (:%20%20
                        (CallFunction|PopulateMap _result))))))
              (:then_1
                (if (not (== (Variables|Default|GetWaveNumber) 0))
                  (Networking|SwitchHasAuthority
                    (:Authority
                      (Utilities|FlowControl|DoOnce false :!label _label
                        (:Completed
                          (Development|PrintString "Clear")
                          (Utilities|FlowControl|Delay 3.0)
                          (if (> (+ (Variables|Default|GetWaveNumber) 1) 3)
                            (Development|PrintString "Finish")
                            (else
                              (Development|PrintString "Ready" true true "(R=0.000000,G=0.660000,B=1.000000,A=1.000000)" 18.0)
                              (Utilities|FlowControl|Delay 18.0)
                              (goto _label Reset))))))))))))))))

(event EventBeginPlay
  (bind _outactors (Actor|GetAllActorsOfClass "/Game/ASM/AIMonster/Spawner/BP_SpawnPoint.BP_SpawnPoint_C"))
  (Variables|Default|SetSpawnList _outactors)
  (Development|PrintString "Ready" true true "(R=0.000000,G=0.660000,B=1.000000,A=1.000000)" 17.0)
  (Utilities|FlowControl|Delay 2e+01)
  (Utilities|Time|SetTimerbyEvent (delegate Custom|ActivateSpawner) (Math|Random|RandomFloatinRange 0.75 1.0) true)
  (CallFunction|PopulateMap (Variables|Default|GetWaveNumber)))

(fn ConstructionScript)

(fn PopulateMap
  (params (WaveNumber :type Integer))
  (bind _returnvalue (Utilities|GetDataTableRow "/Game/ASM/AIMonster/Spawner/DT_WaveDetails.DT_WaveDetails" (Utilities|String|StringToName (Utilities|String|ToString(Integer) WaveNumber)))
    (:then
      (bind _output_get (Variables|Default|SetEnemyList (Utilities|Map|MakeMap "/Game/ASM/AIMonster/Monsters/BP_Goblin.BP_Goblin_C" (.goblin _returnvalue) "/Game/ASM/AIMonster/Monsters/BP_Kobold.BP_Kobold_C" (.kobold _returnvalue) "/Game/ASM/AIMonster/Monsters/BP_Troll.BP_Troll_C" (.troll _returnvalue))))
      (bind _values (Utilities|Map|Values _output_get))
      (for _array_element _values
        (Variables|Default|SetNumberOfEnemies (+ _array_element (Variables|Default|GetNumberOfEnemies)))))))

(fn ChooseEnemy
  (bind _keys (Utilities|Map|Keys (Variables|Default|GetEnemyList) :!label _label))
  (bind _output_get (LocalVariables|SetChosenEnemy (Utilities|Array|Get(acopy) _keys (Math|Random|RandomInteger (Utilities|Array|Length _keys)))))
  (LocalVariables|SetEnemyNumber (.Value (Utilities|Map|Find (Variables|Default|GetEnemyList) _output_get)))
  (if (> (.Value (Utilities|Map|Find (Variables|Default|GetEnemyList) _output_get)) 0)
    (Utilities|Map|Add (Variables|Default|GetEnemyList) (LocalVariables|GetChosenEnemy) (- (LocalVariables|GetEnemyNumber) 1))
    (Variables|Default|SetNumberOfEnemies (- (Variables|Default|GetNumberOfEnemies) 1))
    (return (LocalVariables|GetChosenEnemy))
    (else
      (goto _label))))