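; BP_Spawner is an enemy spawner actor that continuously spawns BP_Goblin monsters in the level.
; Two seconds after BeginPlay, it increments CurrentWave once and starts a looping one-second SpawnWave timer that never gets cleared here.
; Each tick of that timer spawns a goblin at a random BP_Spawner's transform, so every spawner runs its own timer while all share the same spawn points.
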(event Custom|SpawnWave
  (CallFunction|SpawnGoblin))

(event EventBeginPlay
  (Utilities|FlowControl|Delay 2.0)
  (CallFunction|SetupNewWave))

(event Collision|EventActorBeginOverlap
  (params (OtherActor :type Actor%20Object%20Reference)))

(event EventTick
  (params (DeltaSeconds :type Float%20%28single-precision%29)))

(fn ConstructionScript)

(fn SetupNewWave
  (Math|Integer|IncrementInt (Variables|Default|GetCurrentWave)
    (:%20%20
      (Utilities|Time|SetTimerbyFunctionName 0 "SpawnWave" 1.0 true))))

(fn SpawnGoblin
  (bind _spawn_point (CallFunction|GetRandomSpawnPoint))
  (Utilities|IsValid _spawn_point
    (:Is%20Valid
      (Game|SpawnActorfromClass "/Game/ASM/AIMonster/Monsters/BP_Goblin.BP_Goblin_C" (Transformation|GetActorTransform _spawn_point) "Undefined" 0 0))))

(fn GetRandomSpawnPoint
  (bind _outactors (Actor|GetAllActorsOfClass "BP_Spawner_C"))
  (return (Utilities|Array|Get(acopy) _outactors (Math|Random|RandomIntegerinRange 0 (Utilities|Array|LastIndex _outactors)))))