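; BP_MonsterSpawner is a monster wave spawner that runs a start countdown before the first wave.
; On BeginPlay, only the authority counts down from InitailCountDown in a looped short Delay, printing the remaining count through DisplayMessage each step.
; At zero it calls SpawnNextWave, which is an empty stub, so no spawning logic exists yet.
; The Delay is a fraction of a second, so the count runs faster than real seconds.
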(event Custom|Display%20Message
  (params (InString :type String))
  (Development|PrintString InString true true "(R=0.000000,G=0.660000,B=1.000000,A=1.000000)" 1e+01))

(event Custom|Spawn%20Next%20Wave)

(event EventBeginPlay
  (Networking|SwitchHasAuthority
    (:Authority
      (Variables|Default|SetCounter (Variables|Default|GetinitailCountDown))
      (CallFunction|DisplayMessage (Utilities|String|Append "Time until Start" (Utilities|String|ToString(Integer) (Variables|Default|GetCounter))) :!label _label)
      (if (== (Variables|Default|GetCounter) 0)
        (CallFunction|SpawnNextWave)
        (else
          (Utilities|FlowControl|Delay 0.2)
          (Math|Integer|DecrementInt (Variables|Default|GetCounter)
            (:%20%20
              (goto _label))))))))

(fn ConstructionScript)