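; BP_LongdistanceMonster is a ranged AI monster that turns toward the closest player and launches rocks.
; AttackRotateToTarget runs a do-once-gated timeline that blends the actor's yaw toward ClosestPlayer along the shortest path, and StopAttackRotation halts it and resets the gate.
; The longDistanceAttack event spawns BP_Rock at the SpawnProjectile component's world transform.
; TargetToLongerAttack and the Base Damage OnRep are empty.
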(event Custom|longDistanceAttack
  ;[1 1 1] Rotate To Target
  (Game|SpawnActorfromClass "/Game/ASM/Content2/LongerWeapon/BP_Rock.BP_Rock_C" (Transformation|GetWorldTransform (Variables|Default|GetSpawnProjectile)) "Undefined" 0 0))

(event Custom|AttackRotateToTarget
  ;[1 1 1] Rotate To Target
  (Utilities|FlowControl|DoOnce false
    (:Completed
      (bind _새_트랙_0 (Timeline|타임라인 PlayFromStart)
        (:Update
          (Utilities|IsValid (Variables|Default|GetClosestPlayer)
            (:Is%20Valid
              (Transformation|SetActorRotation self (Math|Rotator|Lerp(Rotator) (Math|Rotator|MakeRotator 0.0 0.0 (.yaw (Transformation|GetActorRotation))) (Math|Rotator|MakeRotator 0.0 0.0 (.yaw (Math|Rotator|FindLookatRotation (Transformation|GetActorLocation self) (Transformation|GetActorLocation (Variables|Default|GetClosestPlayer))))) _새_트랙_0 true)))))))))

(event Custom|StopAttackRotation
  ;[1 1 1] Rotate To Target
  (Utilities|FlowControl|Sequence
    (:then_0
      (bind _새_트랙_0 (Timeline|타임라인 Stop)
        (:Update
          (Utilities|IsValid (Variables|Default|GetClosestPlayer)
            (:Is%20Valid
              (Transformation|SetActorRotation self (Math|Rotator|Lerp(Rotator) (Math|Rotator|MakeRotator 0.0 0.0 (.yaw (Transformation|GetActorRotation))) (Math|Rotator|MakeRotator 0.0 0.0 (.yaw (Math|Rotator|FindLookatRotation (Transformation|GetActorLocation self) (Transformation|GetActorLocation (Variables|Default|GetClosestPlayer))))) _새_트랙_0 true)))))))
    (:then_1
      (Utilities|FlowControl|DoOnce false) ; enters at Reset
    )))

(event EventBeginPlay
  (|CallParentFunction) ; 지금 이 노드는 비활성 상태입니다. \n핀을 끌어서 다른 노드를 연결하면 활성화됩니다.
)

(event Collision|EventActorBeginOverlap
  (params (OtherActor :type Actor%20Object%20Reference))
  (|CallParentFunction OtherActor) ; 지금 이 노드는 비활성 상태입니다. \n핀을 끌어서 다른 노드를 연결하면 활성화됩니다.
)

(event EventTick
  (params (DeltaSeconds :type Float%20%28single-precision%29))
  (|CallParentFunction DeltaSeconds) ; 지금 이 노드는 비활성 상태입니다. \n핀을 끌어서 다른 노드를 연결하면 활성화됩니다.
)

(fn ConstructionScript
  (|CallParentFunction))

(fn TargettoLongerAttack
  (params (Object :type Object%20Object%20Reference)))

(fn OnRepBaseDamage)