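; Goblin monster AI character that sets its speed, health and behavior from an enemy details struct and can walk to a fixed destination.
; On the server, a looping timer finds players by distance and starts combat when the closest is within sight range.
; Combat pauses that search and loops move, multicast attack montage, then delay.
; Damage briefly shows a widget health bar; aggro-sphere, pawn-sensing and older chase logic are disconnected.
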(event OnComponentBeginOverlap(AggroSphere)
  (params (OverlappedComponent :type Primitive%20Component%20Object%20Reference) (OtherActor :type Actor%20Object%20Reference) (OtherComp :type Primitive%20Component%20Object%20Reference) (OtherBodyIndex :type Integer) (bFromSweep :type Boolean) (SweepResult :type Hit%20Result%20Structure%20%28by%20ref%29))
  ;[1 1 1] Chase Player / Attack
)

(event OnComponentEndOverlap(AggroSphere)
  (params (OverlappedComponent :type Primitive%20Component%20Object%20Reference) (OtherActor :type Actor%20Object%20Reference) (OtherComp :type Primitive%20Component%20Object%20Reference) (OtherBodyIndex :type Integer))
  ;[1 1 1] Chase Player / Attack
)

(event OnSeePawn(PawnSensing)
  (params (Pawn :type Pawn%20Object%20Reference))
  ;[1 1 1] Chase Closest Player
)

(event Custom|Chase%20Player
  ;[1 1 1] Chase Player / Attack
)

(event Custom|Destination
  ;[1 1 1] Go to Destination
  (Networking|SwitchHasAuthority
    (:Authority
      (AI|AIMoveTo self "-2520.000000,2810.000000,0.000000" 0 5.0 false))))

(event Custom|RotateTowardsTarget
  (bind _returnvalue (Transformation|GetActorRotation))
  (Utilities|FlowControl|DoOnce false
    (:Completed
      (bind _rotationtimeline (Timeline|RotationTimeline PlayFromStart)
        (:Update
          (Utilities|IsValid (Variables|거리|GetClosestPlayer)
            (:Is%20Valid
              (Transformation|SetActorRotation (Math|Rotator|Lerp(Rotator) (Transformation|GetActorRotation) (Math|Rotator|MakeRotator (.roll _returnvalue) (.pitch _returnvalue) (.yaw (Math|Rotator|FindLookatRotation (Transformation|GetActorLocation) (Transformation|GetActorLocation (Variables|거리|GetClosestPlayer))))) _rotationtimeline true)))))))))

(event Custom|Server_FindclosestPlayer
  ;[1 1 1] Chase Closest Player
)

(event Custom|StopRotatingTowardsTarget
  (bind _returnvalue (Transformation|GetActorRotation))
  (Utilities|FlowControl|Sequence
    (:then_0
      (bind _rotationtimeline (Timeline|RotationTimeline Stop)
        (:Update
          (Utilities|IsValid (Variables|거리|GetClosestPlayer)
            (:Is%20Valid
              (Transformation|SetActorRotation (Math|Rotator|Lerp(Rotator) (Transformation|GetActorRotation) (Math|Rotator|MakeRotator (.roll _returnvalue) (.pitch _returnvalue) (.yaw (Math|Rotator|FindLookatRotation (Transformation|GetActorLocation) (Transformation|GetActorLocation (Variables|거리|GetClosestPlayer))))) _rotationtimeline true)))))))
    (:then_1
      (Utilities|FlowControl|DoOnce false) ; enters at Reset
    )))

(event EventBeginPlay
  (Networking|SwitchHasAuthority
    (:Authority
      (bind _aswb_monster_healthbar (Utilities|Casting|CastToWB_MonsterHealthbar (UserInterface|GetUserWidgetObject (Variables|Default|GetWidget))))
      (Variables|/Game/ASM/AIMonster/HUD/WB_MonsterHealthbar.WB_MonsterHealthbar_C|SetOwnerGoblin _aswb_monster_healthbar self)
      (Variables|Default|SetWB_HealthBar _aswb_monster_healthbar)
      (CallFunction|AIMovement)
      (CallFunction|AIStats)
      (CallFunction|AIBehavior)
      (Utilities|Time|SetTimerbyFunctionName 0 "LookForPlayer" 1.0 true))))

(event Custom|ShowHealthBar
  ;[1 1 1] HealthBar
  (Default|ShowHealthBar (Variables|Default|GetWB_HealthBar))
  (Utilities|Time|SetTimerbyEvent (delegate Custom|HideHealthBar) 5.0))

(event Custom|HideHealthBar
  ;[1 1 1] HealthBar
  (Default|HideHealthBar (Variables|Default|GetWB_HealthBar)))

(event Custom|MC_PlayerMontage
  (params (AnimMontage :type Anim%20Montage%20Object%20Reference))
  ;[1 1 1] Play Montage
  (bind _returnvalue (Animation|PlayAnimMontage AnimMontage 1.0 "None"))
  (Variables|Default|SetAttackDelay _returnvalue))

(event Custom|Server_PlayerMontage
  (params (AnimMontage :type Anim%20Montage%20Object%20Reference))
  ;[1 1 1] Play Montage
  (CallFunction|MCPlayerMontage AnimMontage))

(event Custom|initiateCombat
  (Variables|Default|SetHasTarget true)
  (Class|KismetSystemLibrary|PauseTimer 0 "LookForPlayer")
  (if (.TargetClosestPlayer? (Utilities|Struct|BreakS_AIBehaviorDetails (.S_BehaviorDetails (Utilities|Struct|BreakS_AIEnemyDetails (Variables|Default|GetS_EnemyDetails)))))
    (AI|AIMoveTo self "0, 0, 0" (Variables|거리|GetClosestPlayer) 5.0 false
      (:OnSuccess
        _))
    (else
      (AI|AIMoveTo (Variables|거리|GetFurthestPlayer) "0, 0, 0" 0 5.0 false
        (:OnSuccess
          _))))
  (CallFunction|MCPlayerMontage (.Attack01 (Utilities|Struct|BreakS_AIAttackDetails (.S_AttackDetails (Utilities|Struct|BreakS_AIEnemyDetails (Variables|Default|GetS_EnemyDetails))))))
  (Utilities|FlowControl|Delay (Variables|Default|GetAttackDelay))
  (CallFunction|RestartCombat))

(event Custom|RestartCombat
  (if (.TargetClosestPlayer? (Utilities|Struct|BreakS_AIBehaviorDetails (.S_BehaviorDetails (Utilities|Struct|BreakS_AIEnemyDetails (Variables|Default|GetS_EnemyDetails)))))
    (AI|AIMoveTo self "0, 0, 0" (Variables|거리|GetClosestPlayer) 5.0 false
      (:OnSuccess
        _))
    (else
      (AI|AIMoveTo (Variables|거리|GetFurthestPlayer) "0, 0, 0" 0 5.0 false
        (:OnSuccess
          _))))
  (CallFunction|MCPlayerMontage (.Attack01 (Utilities|Struct|BreakS_AIAttackDetails (.S_AttackDetails (Utilities|Struct|BreakS_AIEnemyDetails (Variables|Default|GetS_EnemyDetails))))))
  (Utilities|FlowControl|Delay (Variables|Default|GetAttackDelay))
  (CallFunction|RestartCombat))

(fn ConstructionScript)

(fn AITakeDamage
  (CallFunction|ShowHealthBar)
  (Variables|Default|SetCurrentHealth (- (Variables|Default|GetCurrentHealth) 1e+01)))

(fn OnRepCurrentAttack)

(fn AIMovement
  (Variables|/Script/Engine.CharacterMovementComponent|SetMaxWalkSpeed (Variables|Character|GetCharacterMovement) (Utilities|Struct|BreakS_AIMovementDetails (.S_MovementDetails (Utilities|Struct|BreakS_AIEnemyDetails (Variables|Default|GetS_EnemyDetails))))))

(fn AIStats
  (bind _s_enemydetails (Variables|Default|GetS_EnemyDetails))
  (bind _s_statdetails (Utilities|Struct|BreakS_AIEnemyDetails _s_enemydetails))
  (bind _maxhp (Utilities|Struct|BreakS_AIStatDetails _s_statdetails))
  (Variables|Default|SetMaxHealth _maxhp)
  (Variables|Default|SetCurrentHealth _maxhp))

(fn AIBehavior
  (if (.GotoDestination? (Utilities|Struct|BreakS_AIBehaviorDetails (.S_BehaviorDetails (Utilities|Struct|BreakS_AIEnemyDetails (Variables|Default|GetS_EnemyDetails)))))
    (CallFunction|Destination)))

(fn FindClosestPlayer
  (Variables|거리|SetClosestPlayerDistance 5e+04)
  (Variables|거리|SetFurthestPlayerDistance 1e+02)
  (bind _outactors (Actor|GetAllActorsOfClass "/Game/ASM/Content2/ThirdPerson/Blueprints/BP_ThirdPersonCharacter.BP_ThirdPersonCharacter_C"))
  (for _array_element _outactors
    (if (< (Transformation|GetDistanceTo _array_element self) (Variables|거리|GetClosestPlayerDistance))
      (Variables|거리|SetClosestPlayerDistance (Transformation|GetDistanceTo _array_element self))
      (Variables|거리|SetClosestPlayer _array_element)
      (elif (> (Transformation|GetDistanceTo _array_element self) (Variables|거리|GetFurthestPlayerDistance))
        (Variables|거리|SetFurthestPlayerDistance (Transformation|GetDistanceTo _array_element self))
        (Variables|거리|SetFurthestPlayer _array_element)))))

(fn LookforPlayer
  (CallFunction|FindClosestPlayer)
  (if (< (Transformation|GetDistanceTo (Variables|거리|GetClosestPlayer) self) (.SeePlayerDistance (Utilities|Struct|BreakS_AIBehaviorDetails (.S_BehaviorDetails (Utilities|Struct|BreakS_AIEnemyDetails (Variables|Default|GetS_EnemyDetails))))))
    (CallFunction|InitiateCombat)))