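; Base monster AI pawn, configured by an EnemyDetails struct, that chases players and plays attack montages.
; Aggro overlap with a differing-faction player, or non-lethal damage, starts an AIMoveTo chase of the nearest player class-wide, ignoring PlayersInRange.
; Reaching the target plays Attack01, then re-runs the move after a delay without retargeting, with no Behavior Tree.
; RPC-style events handle montages, speed and death, which destroys the actor after its montage starts.
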(event OnComponentBeginOverlap(AggroCollision)
  (params (OverlappedComponent :type Primitive%20Component%20Object%20Reference) (OtherActor :type Actor%20Object%20Reference) (OtherComp :type Primitive%20Component%20Object%20Reference) (OtherBodyIndex :type Integer) (bFromSweep :type Boolean) (SweepResult :type Hit%20Result%20Structure%20%28by%20ref%29))
  ;[1 1 1] Chase Player
  (bind _asbp_third_person_character (Utilities|Casting|CastToBP_ThirdPersonCharacter OtherActor))
  (Utilities|Array|Add (Variables|Collision|GetPlayersInRange) _asbp_third_person_character)
  (Variables|Collision|SethasAggro true)
  (Variables|Default|SetClosestPlayer _asbp_third_person_character)
  (if (Utilities|Enum|NotEqual(Enum) (.Factions (Utilities|Struct|BreakS_MonsterDetails (Variables|콜리전|GetEnemyDetails))) (Variables|/Game/ASM/Content2/ThirdPerson/Blueprints/BP_ThirdPersonCharacter.BP_ThirdPersonCharacter_C|GetFaction _asbp_third_person_character))
    (CallFunction|ChasePlayer)))

(event OnComponentEndOverlap(AggroCollision)
  (params (OverlappedComponent :type Primitive%20Component%20Object%20Reference) (OtherActor :type Actor%20Object%20Reference) (OtherComp :type Primitive%20Component%20Object%20Reference) (OtherBodyIndex :type Integer))
  ;[1 1 1] Chase Player
  (bind _asbp_third_person_character (Utilities|Casting|CastToBP_ThirdPersonCharacter OtherActor))
  (Utilities|Array|RemoveItem (Variables|Collision|GetPlayersInRange) _asbp_third_person_character))

(event Custom|RestartCombat
  (bind _enemydetails (Variables|콜리전|GetEnemyDetails))
  (bind _closestplayer (Variables|Default|GetClosestPlayer))
  (bind (_name _movementdetails _factions _offensivedetails) (Utilities|Struct|BreakS_MonsterDetails _enemydetails))
  (bind (_maxattacks _attack01) (Utilities|Struct|BreakS_OffensiveDetails _offensivedetails))
  ;[1 1 1] Chase Player
  (AI|AIMoveTo self (Transformation|GetActorLocation _closestplayer) _closestplayer (Variables|콜리전|GetRadius) false
    (:OnSuccess
      (switch int _maxattacks
        (:Default
          (Variables|콜리전|SetCurrentAttack _attack01)
          (CallFunction|MCPlayMontage (Utilities|Struct|BreakS_AttackDetails (Variables|콜리전|GetCurrentAttack)))
          (Utilities|FlowControl|Delay 3.0)
          (CallFunction|RestartCombat))))))

(event Custom|Destination
  ;[1 1 1] Go to Destination
  (AI|AIMoveTo self "0, 0, 0" 0 5.0 false))

(event Custom|ChasePlayer
  (bind _enemydetails (Variables|콜리전|GetEnemyDetails))
  (bind _closestplayer (Variables|Default|GetClosestPlayer))
  (bind (_name _movementdetails _factions _offensivedetails) (Utilities|Struct|BreakS_MonsterDetails _enemydetails))
  (bind (_maxattacks _attack01) (Utilities|Struct|BreakS_OffensiveDetails _offensivedetails))
  ;[1 1 1] Chase Player
  (CallFunction|GetClosestPlayer)
  (CallFunction|ClientSetMovementSpeed (Utilities|Struct|BreakS_MovementDetails _movementdetails))
  (AI|AIMoveTo self (Transformation|GetActorLocation _closestplayer) _closestplayer (Variables|콜리전|GetRadius) false
    (:OnSuccess
      (switch int _maxattacks
        (:Default
          (Variables|콜리전|SetCurrentAttack _attack01)
          (CallFunction|MCPlayMontage (Utilities|Struct|BreakS_AttackDetails (Variables|콜리전|GetCurrentAttack)))
          (Utilities|FlowControl|Delay 3.0)
          (CallFunction|RestartCombat))))))

(event Game|Damage|EventAnyDamage
  (params (Damage :type Float%20%28single-precision%29) (DamageType :type Damage%20Type%20Object%20Reference) (InstigatedBy :type Controller%20Object%20Reference) (DamageCauser :type Actor%20Object%20Reference))
  ;[1 1 1] Damage
  (Variables|Default|SetCurrentHealth (- (Variables|Default|GetCurrentHealth) Damage))
  (if (<= (Variables|Default|GetCurrentHealth) 0.0)
    (Collision|SetCollisionEnabled (Variables|Collision|GetCapsuleComponent) "NoCollision")
    (CallFunction|ServerDeath)
    (else
      (CallFunction|ChasePlayer))))

(event EventBeginPlay
  (CallFunction|SetupEnemyDetails)
  (if (.GotoDestination? (Utilities|Struct|BreakS_BehaviorDetails (.BehaviorDetails (Utilities|Struct|BreakS_MonsterDetails (Variables|콜리전|GetEnemyDetails)))))
    (CallFunction|Destination)))

(fn ConstructionScript)

(fn SetupEnemyDetails
  (Variables|/Script/Engine.CharacterMovementComponent|SetMaxWalkSpeed (Variables|Character|GetCharacterMovement) (Utilities|Struct|BreakS_MovementDetails (.MovementDetails (Utilities|Struct|BreakS_MonsterDetails (Variables|콜리전|GetEnemyDetails))))))

(fn OnRepCurrentAttack)

(fn GetClosestPlayer
  (Variables|Default|SetClosestPlayerDistance 99999999999999.0)
  (bind _outactors (Actor|GetAllActorsOfClass "/Game/ASM/Content2/ThirdPerson/Blueprints/BP_ThirdPersonCharacter.BP_ThirdPersonCharacter_C"))
  (for _array_element _outactors
    (if (< (Transformation|GetDistanceTo _array_element self) (Variables|Default|GetClosestPlayerDistance))
      (Variables|Default|SetClosestPlayerDistance (Transformation|GetDistanceTo _array_element self))
      (Variables|Default|SetClosestPlayer _array_element))))

(fn OnRepMaxHealth)

(fn OnRepCurrentHealth)

(fn OnRepDead?)

(event Custom|Server_PlayMontage
  (params (AnimMontage :type Anim%20Montage%20Object%20Reference))
  ;[1 1 1] Attack Montage
  (CallFunction|MCPlayMontage AnimMontage))

(event Custom|MC_PlayMontage
  (params (AnimMontage :type Anim%20Montage%20Object%20Reference))
  ;[1 1 1] Attack Montage
  (bind _returnvalue (Animation|PlayAnimMontage AnimMontage 0.9 "None"))
  (Variables|콜리전|SetAttackDelay _returnvalue))

(event Custom|Client_SetMovementSpeed
  (params (최대%20걷기%20속도 :type Float%20%28single-precision%29))
  (bind _charactermovement (Variables|Character|GetCharacterMovement))
  ;[1 1 1] Movement
  (bind _output_get (Variables|/Script/Engine.CharacterMovementComponent|SetMaxWalkSpeed _charactermovement 최대%20걷기%20속도))
  (CallFunction|ServerSetMovementSpeed _output_get _charactermovement))

(event Custom|Server_SetMovementSpeed
  (params (최대%20걷기%20속도 :type Float%20%28single-precision%29) (타깃 :type Character%20Movement%20Component%20Object%20Reference))
  ;[1 1 1] Movement
  (Variables|/Script/Engine.CharacterMovementComponent|SetMaxWalkSpeed 타깃 최대%20걷기%20속도))

(event Custom|Server_Death
  ;[1 1 1] Dead
  (if (not (Variables|Default|GetDead?))
    (Variables|Default|SetDead? true)
    (CallFunction|MCPlayMontage (.Dead (Utilities|Struct|BreakS_BehaviorDetails (.BehaviorDetails (Utilities|Struct|BreakS_MonsterDetails (Variables|콜리전|GetEnemyDetails))))))
    (Utilities|FlowControl|Delay 1.0)
    (Actor|DestroyActor)))