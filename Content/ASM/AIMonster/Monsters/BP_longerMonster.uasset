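; BP_longerMonster is an AI monster that chases players and attacks them with montages from long range.
; An aggro-sphere overlap from a different-faction player, or damage taken before aggro, starts a looping move-to with a wide acceptance radius, multicast attack and delay.
; Tick smoothly yaws it toward its target.
; Without aggro, BeginPlay can send it to a hard-coded destination, depending on its behavior details.
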(event OnComponentBeginOverlap(AggroSphere)
  (params (OverlappedComponent :type Primitive%20Component%20Object%20Reference) (OtherActor :type Actor%20Object%20Reference) (OtherComp :type Primitive%20Component%20Object%20Reference) (OtherBodyIndex :type Integer) (bFromSweep :type Boolean) (SweepResult :type Hit%20Result%20Structure%20%28by%20ref%29))
  ;[1 1 1] Chase Player / Attack
  (bind _asbp_third_person_character (Utilities|Casting|CastToBP_ThirdPersonCharacter OtherActor))
  (Utilities|Array|Add (Variables|Default|GetPlayerInRange) _asbp_third_person_character)
  (Variables|Default|SethasAggro true)
  (Variables|Default|SetTarget _asbp_third_person_character)
  (if (Utilities|Enum|NotEqual(Enum) (.Faction (Utilities|Struct|BreakS_Monster_Details (Variables|Default|GetAI_Details))) (Variables|/Game/ASM/Content2/ThirdPerson/Blueprints/BP_ThirdPersonCharacter.BP_ThirdPersonCharacter_C|GetFaction _asbp_third_person_character))
    (CallFunction|ChasePlayer)))

(event OnComponentEndOverlap(AggroSphere)
  (params (OverlappedComponent :type Primitive%20Component%20Object%20Reference) (OtherActor :type Actor%20Object%20Reference) (OtherComp :type Primitive%20Component%20Object%20Reference) (OtherBodyIndex :type Integer))
  ;[1 1 1] Chase Player / Attack
  (bind _asbp_third_person_character (Utilities|Casting|CastToBP_ThirdPersonCharacter OtherActor))
  (Utilities|Array|RemoveItem (Variables|Default|GetPlayerInRange) _asbp_third_person_character))

(event Custom|Chase%20Player
  (bind _ai_details (Variables|Default|GetAI_Details))
  (bind _target (Variables|Default|GetTarget))
  (bind _offensivedetails (Utilities|Struct|BreakS_Monster_Details _ai_details))
  (bind (_maxattacks _attack01) (Utilities|Struct|BreakS_OffensiveDetails _offensivedetails))
  ;[1 1 1] Chase Player / Attack
  (AI|AIMoveTo self (Transformation|GetActorLocation _target) _target 9e+02 false
    (:OnSuccess
      (switch int _maxattacks
        (:Default
          (Variables|Default|SetCurrent%20Attack _attack01)
          (CallFunction|MCAttackPlayer (.AttackAnimation (Utilities|Struct|BreakS_AttackDetails (Variables|Default|GetCurrent%20Attack))))
          (Utilities|FlowControl|Delay 3.0)
          (CallFunction|ChasePlayer))))))

(event Custom|Destination
  ;[1 1 1] Go Destination
  (AI|AIMoveTo self "-2520.000000,2810.000000,0.000000" 0 5.0 false
    (:OnSuccess
      (Utilities|FlowControl|Delay 1.0))))

(event Custom|MC_Attack%20Player
  (params (AnimMontage :type Anim%20Montage%20Object%20Reference))
  ;[1 1 1] Chase Player / Attack
  (bind _returnvalue (Animation|PlayAnimMontage AnimMontage 1.0 "None"))
  (Variables|Default|SetAttackDelay _returnvalue))

(event Custom|Server_Attack%20Player
  (params (AnimMontage :type Anim%20Montage%20Object%20Reference))
  ;[1 1 1] Chase Player / Attack
  (CallFunction|MCAttackPlayer AnimMontage))

(event EventTick
  (params (DeltaSeconds :type Float%20%28single-precision%29))
  (CallFunction|LookingPlayer DeltaSeconds))

(event EventBeginPlay
  (if (not (Utilities|Struct|BreakS_BehaviorDetails (.BehaviorDetails (Utilities|Struct|BreakS_Monster_Details (Variables|Default|GetAI_Details)))))
    (CallFunction|Destination)))

(fn ConstructionScript)

(fn AITakeDamage
  (params (AttackingActor :type BP%20Third%20Person%20Character%20Object%20Reference) (Damage :type Float%20%28double-precision%29))
  (if (not (Variables|Default|GethasAggro))
    (Variables|Default|SethasAggro true)
    (Variables|Default|SetTarget AttackingActor)
    (CallFunction|ChasePlayer)))

(fn OnRepCurrentAttack)

(fn LookingPlayer
  (params (DeltaTime :type Float%20%28single-precision%29))
  (Transformation|SetActorRotation (Math|Rotator|MakeRotator 0.0 0.0 (.yaw (Math|Interpolation|RInterpTo (Transformation|GetActorRotation) (Math|Rotator|FindLookatRotation (Transformation|GetActorLocation) (Transformation|GetActorLocation (Variables|Default|GetTarget))) DeltaTime 5.0)))))