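; BP_Sword is a melee weapon actor that deals fixed point damage to actors its collision overlaps during an active swing window.
; SwordCollision starts disabled, and the TriggerSword and StopTriggerSword events switch it on and off.
; Each overlap calls ReqApplyDamage, labelled as the server damage step, which applies point damage credited to the owning character's controller, using the sword's location for hit data and direction.
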(event OnComponentBeginOverlap(SwordCollision)
  (params (OverlappedComponent :type Primitive%20Component%20Object%20Reference) (OtherActor :type Actor%20Object%20Reference) (OtherComp :type Primitive%20Component%20Object%20Reference) (OtherBodyIndex :type Integer) (bFromSweep :type Boolean) (SweepResult :type Hit%20Result%20Structure%20%28by%20ref%29))
  ;[1 1 1] ApplyDamage
  (CallFunction|ReqApplyDamage OtherActor 15.0 (Variables|Default|GetOwnCharacter) self))

(event Custom|ReqApplyDamage
  (params (DamageGetActor :type Actor%20Object%20Reference) (BaseDamage :type Float%20%28double-precision%29) (InstigatorCharacter :type Character%20Object%20Reference) (DamageCauser :type Actor%20Object%20Reference))
  (bind _returnvalue (Transformation|GetActorLocation))
  ;[1 1 1] Damage Server
  (Game|Damage|ApplyPointDamage DamageGetActor BaseDamage _returnvalue (Collision|MakeHitResult false false 0.1 0.0 _returnvalue _returnvalue "0,0,1" "0,0,1" 0 self (Variables|Default|GetSword)) (Pawn|GetController InstigatorCharacter) DamageCauser))

(event Custom|TriggerSword
  ;[1 1 1] TriggerDamage
  (Collision|SetCollisionEnabled (Variables|Default|GetSwordCollision) "QueryAndPhysics"))

(event Custom|StopTriggerSword
  ;[1 1 1] StopTriggerDamage
  (Collision|SetCollisionEnabled (Variables|Default|GetSwordCollision) "NoCollision"))

(event EventBeginPlay
  ;[1 1 1] StopTriggerDamage
  (Collision|SetCollisionEnabled (Variables|Default|GetSwordCollision) "NoCollision"))

(fn ConstructionScript)