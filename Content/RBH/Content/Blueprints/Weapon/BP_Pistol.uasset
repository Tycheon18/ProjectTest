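; Pistol weapon actor that fires hitscan shots with montages, muzzle effects and sound.
; AttackWeapon1 calls DoShoot, which reloads when empty, adding a full magazine to PistolAmmo.
; For player 0's pawn, it requests ammo use, also decrementing on remote as local prediction, and line-traces ahead of the camera.
; Request events consume ammo and apply damage to the hit actor; OnRep handlers are empty and debug trace and ammo printing remain.
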(event Custom|ReqApplyDamage
  (params (DamagedActor :type Actor%20Object%20Reference%20%28by%20ref%29) (BaseDamage :type Float%20%28single-precision%29) (InstigatorChar :type Character%20Object%20Reference%20%28by%20ref%29) (DamageCauser :type Actor%20Object%20Reference%20%28by%20ref%29))
  (Game|Damage|ApplyDamage DamagedActor BaseDamage (Pawn|GetController InstigatorChar) DamageCauser))

(event Custom|ReqUseAmmo
  (CallFunction|UseAmmo))

(event EventBeginPlay
  (Variables|Default|SetPistolAmmo (Variables|Default|GetMaxPistolAmmo)))

(fn ConstructionScript)

(fn OnRepAmmo)

(fn DoShoot
  (bind _returnvalue (Game|GetPlayerCameraManager 0))
  (bind _pistolbody (Variables|Default|GetPistolBody))
  (bind _returnvalue_2 (Transformation|GetActorForwardVector _returnvalue))
  (bind _returnvalue_3 (Transformation|GetActorLocation _returnvalue))
  (if (> (Variables|Default|GetPistolAmmo) 0)
    ;[1 1 1] Gun_Fire_VFX
    (Effects|SpawnEmitteratLocation "/Game/RBH/Content2/StarterContent/Particles/P_Explosion.P_Explosion" (Transformation|GetSocketLocation _pistolbody "muzzle") (Transformation|GetSocketRotation _pistolbody "muzzle") "0.080000,0.080000,0.080000")
    ;[1 1 1] Gun_Fire_SFX
    (Audio|SpawnSoundatLocation "/Game/RBH/Content2/StarterContent/Audio/Explosion01.Explosion01" (Transformation|GetActorLocation) "0, 0, 0" 1.0 1.0 0.0 0 0)
    ;[1 1 1] CheckPlayer
    (if (== (Variables|Character|GetOwnCharacter) (Game|GetPlayerCharacter 0))
      (CallFunction|ReqUseAmmo)
      (Networking|SwitchHasAuthority
        (:Authority
          _)
        (:Remote
          (Variables|Default|SetPistolAmmo (- (Variables|Default|GetPistolAmmo) 1))))
      ;[1 1 1] SetDamage
      (bind _outhit (Collision|LineTraceForObjects (+ _returnvalue_3 (* _returnvalue_2 4e+02)) (+ _returnvalue_3 (* _returnvalue_2 8e+02)) (Utilities|Array|MakeArray "ObjectTypeQuery1" "ObjectTypeQuery2" "ObjectTypeQuery3" "ObjectTypeQuery4" "ObjectTypeQuery5" "ObjectTypeQuery6" "ObjectTypeQuery7") false (Utilities|Array|MakeArray (Variables|Character|GetOwnCharacter) 0 0) "ForDuration"))
      (CallFunction|ReqApplyDamage (.HitActor (Collision|BreakHitResult _outhit)) (Variables|Default|GetPistolDamage) (Variables|Character|GetOwnCharacter) self))
    (else
      (CallFunction|DoReload))))

(fn AttackWeapon1
  (Animation|PlayAnimMontage (Variables|Character|GetOwnCharacter) "/Game/RBH/Content2/Characters/Mannequins/Animations/RifleAnimPro/InPlace/Rifle_ShootOnce_Montage.Rifle_ShootOnce_Montage" 1.7 "None")
  (CallFunction|DoShoot))

(fn UseAmmo
  (bind _output_get (Variables|Default|SetPistolAmmo (- (Variables|Default|GetPistolAmmo) 1)))
  (Development|PrintString (Utilities|String|Append "Ammo" (Utilities|String|ToString(Integer) _output_get)) true true "(R=0.000000,G=0.660000,B=1.000000,A=1.000000)" 3.0)
  (return _output_get))

(fn OnRepPistolAmmo)

(fn DoReload
  (Animation|PlayAnimMontage (Variables|Character|GetOwnCharacter) "/Game/RBH/Content2/Characters/Mannequins/Animations/RifleAnimPro/InPlace/Rifle_Reload_Montage.Rifle_Reload_Montage" 1.0 "None")
  (Variables|Default|SetPistolAmmo (+ (Variables|Default|GetPistolAmmo) (Variables|Default|GetMaxPistolAmmo))))