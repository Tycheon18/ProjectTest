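; BP_Pistol is a pistol weapon blueprint tied to a DwarfGunner character, providing firing effects and an attack animation.
; DoShoot spawns a scaled-down muzzle emitter at the PistolBody socket and a gunshot sound at the actor, then ends on an empty local-player check.
; AttackWeapon1 plays the PistolAttack1 montage on the gunner with a debug print.
; Ammo starts at zero on BeginPlay; its OnRep handler is empty, and no shot logic uses it.
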(event EventBeginPlay
  (Variables|Default|SetAmmo 0))

(fn ConstructionScript)

(fn OnRepAmmo)

(fn DoShoot
  (bind _pistolbody (Variables|Default|GetPistolBody))
  ;[1 1 1] Gun_Fire_VFX
  (Effects|SpawnEmitteratLocation 0 (Transformation|GetSocketLocation _pistolbody "muzzle") (Transformation|GetSocketRotation _pistolbody "muzzle") "0.100000,0.100000,0.100000")
  ;[1 1 1] Gun_Fire_SFX
  (Audio|SpawnSoundatLocation 0 (Transformation|GetActorLocation) "0, 0, 0" 1.0 1.0 0.0 0 0)
  (if (== (Variables|Character|GetDwarfGunner) (Game|GetPlayerCharacter 0))
    _))

(fn AttackWeapon1
  (Animation|PlayAnimMontage (Variables|Character|GetDwarfGunner) 0 1.0 "None") ; PistolAttack1
  (Development|PrintString "PistolAttack1" true true "(R=0.000000,G=0.660000,B=1.000000,A=1.000000)" 2e+01))