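; Playable Knight character that spawns a sword and shield on its hand sockets and supports attack, block and dash skill.
; Blocking slows movement, shows an energy shield and adds DefensivePower to incoming damage before the parent handles it.
; The stamina-gated, grounded dash boosts movement, locks input and uses a timeline for forward motion and camera FOV, with Niagara FX.
; During the dash, DashBarrier overlaps send point-damage requests through ReqApplyDamage.
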(event EventBeginPlay
  (|CallParentFunction)
  (CallFunction|EquipWeapon) ; SetEquipWeapon
  ;[1 1 1] DashSetting
  (Collision|SetCollisionEnabled (Variables|Default|GetDashBarrier) "NoCollision") ; DashBarrierNoCollision
  (Rendering|SetVisibility (Variables|Default|GetEnergyShield) false false) ; NoneVisibleEnergyShield,DashBarrier
  (CallFunction|DefaultDashSetup)
  (Components|Timeline|SetPlayRate (Variables|Default|GetDashTimeLine) (Variables|Skill|GetDashRate))
  (Variables|Skill|SetDashRate (* (Variables|Skill|GetDashDistance) (Variables|Skill|GetDashRate))))

(event OnComponentBeginOverlap(DashBarrier)
  (params (OverlappedComponent :type Primitive%20Component%20Object%20Reference) (OtherActor :type Actor%20Object%20Reference) (OtherComp :type Primitive%20Component%20Object%20Reference) (OtherBodyIndex :type Integer) (bFromSweep :type Boolean) (SweepResult :type Hit%20Result%20Structure%20%28by%20ref%29))
  (bind _self self)
  ;[1 1 1] UseSkill
  ;;[1 1 1] ApplySkillDamage
  (CallFunction|ReqApplyDamage OtherActor 1e+02 _self _self))

(event Custom|ReqApplyDamage
  (params (DamageGetActor :type Actor%20Object%20Reference) (BaseDamage :type Float%20%28double-precision%29) (InstigatorCharacter :type Character%20Object%20Reference) (DamageCauser :type Actor%20Object%20Reference))
  ;[1 1 1] UseSkill
  ;;[1 1 1] SkillDamageServer
  (for _array_element (Collision|GetOverlappingActors (Variables|Default|GetDashBarrier) "/Game/ASM/AIMonster/Monsters/BP_MasterMonster.BP_MasterMonster_C" :!class /Script/Engine.PrimitiveComponent)
    (Game|Damage|ApplyPointDamage DamageGetActor BaseDamage (Transformation|GetActorLocation _array_element) (Collision|MakeHitResult false false 0.0 0.0 (Transformation|GetActorLocation _array_element) (Transformation|GetActorLocation _array_element) "0,0,1" "0,0,1" 0 self (Variables|Default|GetDashBarrier)) (Pawn|GetController InstigatorCharacter) DamageCauser)))

(event EventResUseWeapon2
  (params (IsPress :type Boolean))
  ;[1 1 1] ShieldDefense
  (if IsPress
    (CallFunction|DefensePose)
    (Variables|Movement|SetWeapon2IsPress true)
    (else
      (CallFunction|NoneDefensePose)
      (Variables|Movement|SetWeapon2IsPress false))))

(event Game|Damage|EventAnyDamage
  (params (Damage :type Float%20%28single-precision%29) (DamageType :type Damage%20Type%20Object%20Reference) (InstigatedBy :type Controller%20Object%20Reference) (DamageCauser :type Actor%20Object%20Reference))
  ;[1 1 1] AnyDamage
  (bind _damageout (CallFunction|DoDefense (Variables|Movement|GetIs%20Defensed) Damage))
  (|CallParentFunction _damageout DamageType InstigatedBy DamageCauser))

(event EventResUseSkill
  (params (IputType :type EN_InputType%20Enum :default "NewEnumerator0"))
  (bind _fxlocation (Variables|Default|GetFXLocation))
  (bind _dashbarrier (Variables|Default|GetDashBarrier))
  (bind _dashbarrier_2 (Variables|Default|GetDashBarrier))
  ;[1 1 1] UseSkill
  ;;[1 1 1] CheckFalling
  (if (not (Utilities|IsFalling))
    (bind _canuseskill (CallFunction|UseSkillStamina))
    (if _canuseskill
      (CallFunction|NoneDefensePose)
      ;;[1 1 1] StartDash
      (CallFunction|DashSetup (Variables|Skill|GetDashSpeed) 1e+16 "0.000000,10000000000000000.000000,0.000000" true)
      (Utilities|FlowControl|Delay 0.1)
      (Input|DisableInput (Game|GetPlayerController 0))
      ;;[1 1 1] SpawnParticle, DashBarrier
      (Rendering|SetVisibility _dashbarrier_2 true false)
      (Collision|SetCollisionEnabled _dashbarrier_2 "QueryAndPhysics") ; DashBarrierCollision
      (bind _returnvalue (Niagara|SpawnSystemAttached "/Game/RBH/Content/Texture/DashFX/NG_DashFX.NG_DashFX" _fxlocation "None" (Transformation|GetWorldLocation _fxlocation) (Math|Rotator|MakeRotator 0.0 0.0 (.yaw (Math|Rotator|MakeRotfromX (Transformation|GetActorForwardVector)))) "KeepWorldPosition" true))
      (Variables|Default|SetDashFX _returnvalue)
      (bind _viewvalue (Timeline|DashTimeLine PlayFromStart)
        (:Update
          ;;[1 1 1] DashCameraSetting
          (Pawn|Input|AddMovementInput (Transformation|GetActorForwardVector) 1.0 false)
          (Camera|SetFieldOfView (Variables|Default|GetFollowCamera) (Math|Float|Lerp 9e+01 1e+02 _viewvalue)))
        (:Finished
          ;;[1 1 1] EndDash
          (CallFunction|DashSetup (Variables|Movement|GetMax%20Walk%20Speed) (Variables|Movement|GetMax%20Acceleration) (Variables|Movement|GetRotation%20Rate) true)
          (Rendering|SetVisibility _dashbarrier false false)
          (Collision|SetCollisionEnabled _dashbarrier "NoCollision") ; DashBarrierNoCollision
          (Input|EnableInput (Game|GetPlayerController 0))
          (Components|Activation|Deactivate (Variables|Default|GetDashFX)))))))

(event EventResRunning
  (params (IsPress :type Boolean))
  ;[1 1 1] DefenseRunning
  (if (Variables|Movement|GetIs%20Defensed)
    (Variables|/Script/Engine.CharacterMovementComponent|SetMaxWalkSpeed (Variables|Character|GetCharacterMovement) 2.5e+02)
    (CallFunction|EventAddStamina)
    (else
      (CallFunction|DoRunning))))

(event EventResWalking
  (params (IsPress :type Boolean))
  ;[1 1 1] DefenseWalking
  (if (Variables|Movement|GetIs%20Defensed)
    (Variables|/Script/Engine.CharacterMovementComponent|SetMaxWalkSpeed (Variables|Character|GetCharacterMovement) 2.5e+02)
    (CallFunction|EventAddStamina)
    (else
      (CallFunction|DoWalking))))

(event EventResUseWeapon1
  (params (IsPress :type Boolean))
  ;[1 1 1] SwordAttackMotion
  (if IsPress
    (Utilities|FlowControl|DoOnce false :!label _label
      (:Completed
        (CallFunction|NoneDefensePose)
        (bind _returnvalue (Animation|PlayAnimMontage "/Game/RBH/Content2/Characters/Mannequins/Animations/KnightAnim/InPlace/SwordSlash_Montage.SwordSlash_Montage" 1.0 "None"))
        (Utilities|FlowControl|Delay _returnvalue)
        (if (Variables|Movement|GetWeapon2IsPress)
          (CallFunction|DefensePose)
          (goto _label Reset)
          (else
            (CallFunction|NoneDefensePose)
            (goto _label Reset)))))))

(fn ConstructionScript
  (|CallParentFunction))

(fn EquipWeapon
  (bind _mesh (Variables|Character|GetMesh))
  (bind _mesh_2 (Variables|Character|GetMesh))
  (bind _righthandsocket (Variables|Equipment|GetRightHandSocket))
  (bind _lefthandsocket (Variables|Equipment|GetLeftHandSocket))
  (Utilities|FlowControl|Sequence
    (:then_0
      ;[1 1 1] SynchronizeControllerRotation
      (bind _asabp_knight (Utilities|Casting|CastToABP_Knight (Components|SkeletalMesh|GetAnimInstance (Variables|Character|GetMesh))))
      (bind _output_get (Variables|/Game/RBH/Content2/Characters/Mannequins/Animations/ABP_Knight.ABP_Knight_C|SetIsEquip _asabp_knight true))
      (Variables|Default|SetbUseControllerRotationYaw _output_get))
    (:then_1
      ;[1 1 1] EquipRightHand(Sword)
      (bind _returnvalue (Game|SpawnActorfromClass "/Game/RBH/Content/Blueprints/Weapon/BP_Sword.BP_Sword_C" (Transformation|GetSocketTransform _mesh_2 _righthandsocket "RTS_World") "Undefined" 0 self 0 0))
      (bind _output_get_2 (Variables|Equipment|SetSword _returnvalue))
      (Transformation|AttachComponentToComponent _output_get_2 _mesh_2 _righthandsocket "SnapToTarget" "SnapToTarget" "SnapToTarget" true))
    (:then_2
      ;[1 1 1] EquipLeftHand(Shield)
      (bind _returnvalue_2 (Game|SpawnActorfromClass "/Game/RBH/Content/Blueprints/Weapon/BP_Shield.BP_Shield_C" (Transformation|GetSocketTransform _mesh _lefthandsocket "RTS_World") "Undefined" 0 self 0 0))
      (bind _output_get_3 (Variables|Equipment|SetShield _returnvalue_2))
      (Transformation|AttachComponentToComponent _output_get_3 _mesh _lefthandsocket "SnapToTarget" "SnapToTarget" "SnapToTarget" true))))

(fn OnRepIsDefensed)

(fn DoDefense
  (params (IsDefensed :type Boolean) (DamageIN :type Float%20%28double-precision%29))
  (if IsDefensed
    (bind _output_get (Variables|Equipment|SetDefensivePower (Variables|Equipment|GetDefensivePower)))
    (return (+ _output_get DamageIN))
    (else
      (return DamageIN))))

(fn DefensePose
  (Animation|PlayAnimMontage "/Game/RBH/Content2/Characters/Mannequins/Animations/KnightAnim/InPlace/Idle_Block_MSA_Montage.Idle_Block_MSA_Montage" 1.0 "None")
  (Variables|Movement|SetIs%20Defensed true)
  (Rendering|SetVisibility (Variables|Default|GetEnergyShield) true false)
  (Variables|/Script/Engine.CharacterMovementComponent|SetMaxWalkSpeed (Variables|Character|GetCharacterMovement) 2.5e+02))

(fn NoneDefensePose
  (Animation|StopAnimMontage "/Game/RBH/Content2/Characters/Mannequins/Animations/KnightAnim/InPlace/Idle_Block_MSA_Montage.Idle_Block_MSA_Montage")
  (Variables|Movement|SetIs%20Defensed false)
  (Rendering|SetVisibility (Variables|Default|GetEnergyShield) false false)
  (CallFunction|DoWalking))

(fn DashSetup
  (params (Max%20Walk%20Speed :type Float%20%28single-precision%29) (Max%20Acceleration :type Float%20%28single-precision%29) (Rotation%20Rate :type Rotator) (bNewVisibility :type Boolean))
  (bind _charactermovement (Variables|Character|GetCharacterMovement))
  ;[1 1 1] SetDash
  (Variables|/Script/Engine.CharacterMovementComponent|SetMaxWalkSpeed _charactermovement Max%20Walk%20Speed)
  (Variables|/Script/Engine.CharacterMovementComponent|SetMaxAcceleration _charactermovement Max%20Acceleration)
  (Variables|/Script/Engine.CharacterMovementComponent|SetRotationRate _charactermovement Rotation%20Rate)
  ;[1 1 1] SetKnightVisibility
  (Rendering|SetVisibility (Variables|Character|GetMesh) bNewVisibility false)
  (bind _asbp_sword (Utilities|Casting|CastToBP_Sword (Variables|Equipment|GetSword)))
  (Rendering|SetVisibility (Variables|/Game/RBH/Content/Blueprints/Weapon/BP_Sword.BP_Sword_C|GetSword _asbp_sword) bNewVisibility false)
  (bind _asbp_shield (Utilities|Casting|CastToBP_Shield (Variables|Equipment|GetShield)))
  (Rendering|SetVisibility (Variables|/Game/RBH/Content/Blueprints/Weapon/BP_Shield.BP_Shield_C|GetShield _asbp_shield) bNewVisibility false)
  (return))

(fn DefaultDashSetup
  (bind _charactermovement (Variables|Character|GetCharacterMovement))
  (Variables|Movement|SetMax%20Walk%20Speed (Variables|/Script/Engine.CharacterMovementComponent|GetMaxWalkSpeed _charactermovement))
  (Variables|Movement|SetMax%20Acceleration (Variables|/Script/Engine.CharacterMovementComponent|GetMaxAcceleration _charactermovement))
  (Variables|Movement|SetRotation%20Rate (Variables|/Script/Engine.CharacterMovementComponent|GetRotationRate _charactermovement)))

(fn UseSkillStamina
  (bind _skillstamina (Variables|Skill|GetSkillStamina))
  (bind _asbp_team_3player_state (Utilities|Casting|CastToBP_Team3PlayerState (Variables|Default|GetPlayerState)))
  (if (> (- (Variables|/Game/RBH/Content/PlayableCharater/BP_Team3PlayerState.BP_Team3PlayerState_C|GetCurrentStamina _asbp_team_3player_state) _skillstamina) 0.0)
    (Default|UseStamina _asbp_team_3player_state _skillstamina)
    (return true)
    (else
      (return false))))