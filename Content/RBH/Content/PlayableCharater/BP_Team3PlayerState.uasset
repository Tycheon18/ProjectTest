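; Player state Blueprint that holds a player's health, stamina, coins and death flag, filling health and stamina to their maximums on BeginPlay.
; Functions apply clamped damage, healing and stamina changes or add coins, with damage reporting only the killing hit and stamina changes reporting depletion.
; RepNotify handlers rebroadcast health, stamina and coin changes through event dispatchers, while the death flag's handler is empty.
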(event EventBeginPlay
  (Variables|PlayerState|SetCurrentHP (Variables|PlayerState|GetMaxHP))
  (Variables|PlayerState|SetCurrentStamina (Variables|PlayerState|GetMaxStamina)))

(fn ConstructionScript)

(fn AddDamage
  (params (DamageIN :type Float%20%28double-precision%29))
  (if (> (Variables|PlayerState|GetCurrentHP) 0.0)
    (bind _output_get (Variables|PlayerState|SetCurrentHP (Math|Float|Clamp(Float) (- (Variables|PlayerState|GetCurrentHP) DamageIN) 0.0 (Variables|PlayerState|GetMaxHP))))
    (if (> _output_get 0.0)
      (bind _output_get_2 (Variables|Default|SetYouDied false))
      (return _output_get_2)
      (else
        (bind _output_get_3 (Variables|Default|SetYouDied true))
        (return _output_get_3)))
    (else
      (bind _output_get_4 (Variables|Default|SetYouDied false))
      (return _output_get_4))))

(fn AddHeal
  (params (AddHeal :type Float%20%28double-precision%29))
  (Variables|PlayerState|SetCurrentHP (Math|Float|Clamp(Float) (+ (Variables|PlayerState|GetCurrentHP) AddHeal) 0.0 (Variables|PlayerState|GetMaxHP))))

(fn OnRepCurrentHP
  (Default|CallEventDispatcherUpdateHP (Variables|PlayerState|GetCurrentHP) (Variables|PlayerState|GetMaxHP)))

(fn UseStamina
  (params (UseStamina :type Float%20%28double-precision%29))
  (bind _output_get (Variables|PlayerState|SetCurrentStamina (Math|Float|Clamp(Float) (- (Variables|PlayerState|GetCurrentStamina) UseStamina) 0.0 (Variables|PlayerState|GetMaxStamina))))
  (if (> _output_get 0.0)
    (return false)
    (else
      (return true))))

(fn OnRepCurrentStamina
  (Default|CallEventDispatcherUpdateStamina (Variables|PlayerState|GetCurrentStamina) (Variables|PlayerState|GetMaxStamina)))

(fn AddStamina
  (params (AddStamina :type Float%20%28double-precision%29))
  (bind _output_get (Variables|PlayerState|SetCurrentStamina (Math|Float|Clamp(Float) (+ (Variables|PlayerState|GetCurrentStamina) AddStamina) 0.0 (Variables|PlayerState|GetMaxStamina))))
  (if (> _output_get 0.0)
    (return false)
    (else
      (return true))))

(fn OnRepCoin
  (Default|CallEventDispatcherCoin (Variables|PlayerState|GetCoin)))

(fn AddCoin
  (params (Coin :type Integer))
  (Variables|PlayerState|SetCoin (+ Coin (Variables|PlayerState|GetCoin))))

(fn OnRepYouDied)