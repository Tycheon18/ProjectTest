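; BP_Team3Player_Gunner is a playable Gunner character that extends a parent player class and starts with its weapon equipped.
; On BeginPlay it runs the parent logic, then calls DoEquipWeapon with true.
; DoEquipWeapon sets IsEquip on the mesh's ABP_Gunner anim instance and mirrors that value to UseControllerRotationYaw, so the character turns with the controller while armed.
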(event EventBeginPlay
  (|CallParentFunction)
  (CallFunction|DoEquipWeapon true))

(event EventTick
  (params (DeltaSeconds :type Float%20%28single-precision%29))
  (|CallParentFunction DeltaSeconds) ; This node is disabled and will not be called.\nDrag off pins to build functionality.
)

(fn ConstructionScript
  (|CallParentFunction))

(fn DoEquipWeapon
  (params (IsEquip :type Boolean))
  (bind _asabp_gunner (Utilities|Casting|CastToABP_Gunner (Components|SkeletalMesh|GetAnimInstance (Variables|Character|GetMesh))))
  (bind _output_get (Variables|/Game/RBH/Content2/Characters/Mannequins/Animations/ABP_Gunner.ABP_Gunner_C|SetIsEquip _asabp_gunner IsEquip))
  (Variables|Default|SetbUseControllerRotationYaw _output_get))