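; BP_CrystalTower is a tower actor with hit points that monsters wear down on contact.
; Any BP_MasterMonster overlapping its sphere is destroyed and costs the tower one HP, and the tower destroys itself when HP equals zero.
; Tick spins three rune circle meshes on different axes at a fixed per-frame step and copies current HP into GM_SpawnGameMode.
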(event OnComponentBeginOverlap(Sphere)
  (params (OverlappedComponent :type Primitive%20Component%20Object%20Reference) (OtherActor :type Actor%20Object%20Reference) (OtherComp :type Primitive%20Component%20Object%20Reference) (OtherBodyIndex :type Integer) (bFromSweep :type Boolean) (SweepResult :type Hit%20Result%20Structure%20%28by%20ref%29))
  ;[1 1 1] 몬스터가 오버랩 되면 타워 HP 감소, 0이 되면 파괴
  (bind _asbp_master_monster (Utilities|Casting|CastToBP_MasterMonster OtherActor))
  (Actor|DestroyActor _asbp_master_monster)
  (if true
    (bind _output_get (Variables|Default|SetCrystalTowerHP (- (Variables|Default|GetCrystalTowerHP) 1)))
    (Utilities|FlowControl|Sequence
      (:then_0
        (if (== 0 _output_get)
          (Actor|DestroyActor))))))

(event EventTick
  (params (DeltaSeconds :type Float%20%28single-precision%29))
  ;[1 1 1] 구체 주위를 맴도는 구조물 회전값 적용
  (Transformation|AddRelativeRotation (Variables|Default|GetSM_Temple_Rune_Circle_01) "0.000000,1.000000,1.000000" false false)
  (Transformation|AddRelativeRotation (Variables|Default|GetSM_Temple_Rune_Circle_02) "-1.000000,0.000000,-1.000000" false false)
  (Transformation|AddRelativeRotation (Variables|Default|GetSM_Temple_Rune_Circle_03) "0.000000,1.000000,-1.000000" false false)
  (bind _asgm_spawn_game_mode (Utilities|Casting|CastToGM_SpawnGameMode (Game|GetGameMode)))
  (Variables|/Game/ASM/AIMonster/Spawner/GM_SpawnGameMode.GM_SpawnGameMode_C|SetCrystalTowerCurHp _asgm_spawn_game_mode (Variables|Default|GetCrystalTowerHP)))

(fn ConstructionScript)