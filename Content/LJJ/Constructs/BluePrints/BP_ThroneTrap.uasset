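; BP_ThroneTrap is a trap Blueprint, apparently an unfinished draft meant to slow and damage enemies.
; Its Box begin-overlap event gates the logic behind placeholder tag checks on the overlapping actor, using "None" and unwired false inputs.
; It subtracts SlowEnemy from the Enemy's max speed without setting movement speed, then under a repeated check applies fixed damage with no target wired and stores the result in EnemyHP.
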(event OnComponentBeginOverlap(Box)
  (params (OverlappedComponent :type Primitive%20Component%20Object%20Reference) (OtherActor :type Actor%20Object%20Reference) (OtherComp :type Primitive%20Component%20Object%20Reference) (OtherBodyIndex :type Integer) (bFromSweep :type Boolean) (SweepResult :type Hit%20Result%20Structure%20%28by%20ref%29))
  (bind _returnvalue (Actor|ActorHasTag OtherActor "None"))
  (bind _returnvalue_2 (Math|Boolean|ORBoolean _returnvalue false false))
  (if _returnvalue_2
    (Variables|Default|SetSlowEnemy (- (Class|MovementComponent|GetMaxSpeed (Variables|/Script/Engine.Character|GetCharacterMovement (Variables|Default|GetEnemy))) (Variables|Default|GetSlowEnemy)))
    (if _returnvalue_2
      (bind _returnvalue_3 (Game|Damage|ApplyDamage 0 1e+01 0 0))
      (Variables|Default|SetEnemyHP _returnvalue_3))))

(event EventBeginPlay)

(event Collision|EventActorBeginOverlap
  (params (OtherActor :type Actor%20Object%20Reference)))

(event EventTick
  (params (DeltaSeconds :type Float%20%28single-precision%29)))

(fn ConstructionScript)