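; Automated catapult turret that targets nearby pawns and fires flame turret bullets from two guns.
; Each tick, a sphere overlap picks the closest pawn in line of sight, and the head rotates toward it at a constant rate.
; Once the fire interval has passed and a dot product confirms alignment, it shoots.
; A self-re-entering DoN with delays staggers each burst into two alternating rounds from both gun sockets.
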(event Custom|Shoot
  (Variables|Private|SetTimeOfLastShoot (Utilities|Time|GetGameTimeinSeconds))
  (Utilities|FlowControl|Sequence
    (:then_0
      (goto _label Reset))
    (:then_1
      (Utilities|FlowControl|DoN 2 :!label _label
        (:Exit
          (Development|PrintString "Shoot")
          (Game|SpawnActorfromClass "/Game/LJJ/Constructs/BluePrints/BP_FlameTurretBullet.BP_FlameTurretBullet_C" (Transformation|GetSocketTransform (Variables|Default|GetTu_Gun1) "ShootSocket" "RTS_World") "Undefined" 0 0)
          (Utilities|FlowControl|Delay 0.2)
          (Game|SpawnActorfromClass "/Game/LJJ/Constructs/BluePrints/BP_FlameTurretBullet.BP_FlameTurretBullet_C" (Transformation|GetSocketTransform (Variables|Default|GetTu_Gun) "ShootSocket" "RTS_World") "Undefined" 0 0)
          (Utilities|FlowControl|Delay 0.2)
          (goto _label))))))

(event EventTick
  (params (DeltaSeconds :type Float%20%28single-precision%29))
  (Private|FindTarget)
  (Variables|Private|GetTarget
    (:then
      (Private|UpdateTurretRotation DeltaSeconds)
      (Private|UpdateShoot))
    (:else)))

(fn ConstructionScript)

(fn FindTarget
  (LocalVariables|SetBestDistance%28Local%29 (+ (Variables|Default|GetSensingRange) 1.0))
  (bind _outactors (Collision|SphereOverlapActors (Transformation|GetActorLocation) (Variables|Default|GetSensingRange) (Utilities|Array|MakeArray "ObjectTypeQuery3") "/Script/Engine.Actor"))
  (for _array_element _outactors
    (bind _output_get (LocalVariables|SetCurrentTaget%28Local%29 _array_element))
    (bind _output_get_2 (LocalVariables|SetCurrentDistance%28Local%29 (Transformation|GetDistanceTo _output_get self)))
    (if (or (< _output_get_2 (LocalVariables|GetBestDistance%28Local%29)) (not (Utilities|IsValid (LocalVariables|GetBestTarget%28Local%29))))
      (CallFunction|HasLineOfSight (Transformation|GetWorldLocation (Variables|Default|GetTu_Head)) (Transformation|GetActorLocation (LocalVariables|GetCurrentTaget%28Local%29)) (Utilities|Array|MakeArray self (LocalVariables|GetCurrentTaget%28Local%29)))
      (if true
        (LocalVariables|SetBestTarget%28Local%29 (LocalVariables|GetCurrentTaget%28Local%29))
        (LocalVariables|SetBestDistance%28Local%29 (LocalVariables|GetCurrentDistance%28Local%29)))))
  (Variables|Private|SetTarget (LocalVariables|GetBestTarget%28Local%29)))

(fn UpdateTurretRotation
  (params (DeltaSeconds :type Float%20%28double-precision%29))
  (Transformation|SetWorldRotation (Variables|Default|GetTu_Head) (Class|KismetMathLibrary|RInterptoConstant (Transformation|GetWorldRotation (Variables|Default|GetTu_Head)) (Math|Rotator|FindLookatRotation (Transformation|GetWorldLocation (Variables|Default|GetTu_Head)) (Transformation|GetActorLocation (Variables|Private|GetTarget))) DeltaSeconds (Variables|constants|GetInterp%20Speed)) false false))

(fn UpdateShoot
  (if (> (- (Utilities|Time|GetGameTimeinSeconds) (Variables|Private|GetTimeOfLastShoot)) (Variables|Private|GetRateOfShoot))
    (if (> (Math|Vector|DotProduct (Math|Vector|GetUnitDirection(Vector) (Transformation|GetWorldLocation (Variables|Default|GetTu_Head)) (Transformation|GetActorLocation (Variables|Private|GetTarget))) (Math|Vector|GetForwardVector (Variables|Default|GetTu_Head))) 0.99)
      (CallFunction|Shoot))))