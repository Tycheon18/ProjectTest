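; An automated twin-barrel turret that attacks nearby BP_MasterMonster enemies with flame bullets.
; Each tick it picks the nearest monster in sensing range with line of sight and rotates its top toward it at constant speed.
; Once the fire interval elapses and a dot-product check confirms aim, a DoN loop with delays spawns a burst alternating between left and right barrel sockets.
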(event Custom|Fire
  (Variables|Private|SetTimeOfLastFire (Utilities|Time|GetGameTimeinSeconds))
  (Utilities|FlowControl|Sequence
    (:then_0
      (goto _label Reset))
    (:then_1
      (Utilities|FlowControl|DoN 4 :!label _label
        (:Exit
          (Game|SpawnActorfromClass "/Game/LJJ/Constructs/BluePrints/BP_FlameTurretBullet.BP_FlameTurretBullet_C" (Transformation|GetSocketTransform (Variables|Default|GetTurretBarrel-L) "FireSocket" "RTS_World") "Undefined" 0 0)
          (Utilities|FlowControl|Delay 0.2)
          (Game|SpawnActorfromClass "/Game/LJJ/Constructs/BluePrints/BP_FlameTurretBullet.BP_FlameTurretBullet_C" (Transformation|GetSocketTransform (Variables|Default|GetTurretBarrel-R) "FireSocket" "RTS_World") "Undefined" 0 0)
          (Utilities|FlowControl|Delay 0.2)
          (goto _label))))))

(event EventTick
  (params (DeltaSeconds :type Float%20%28single-precision%29))
  (CallFunction|FindBestTarget 0.0)
  (Variables|Private|GetTarget
    (:then
      (CallFunction|UpdateTurretRotation DeltaSeconds)
      (CallFunction|UpdateFire))
    (:else)))

(fn ConstructionScript)

(fn FindBestTarget
  (params (DeltaSeconds :type Float%20%28double-precision%29))
  (LocalVariables|SetBestDistance%28Local%29 (+ (Variables|Constants|GetSensingRange) 1.0))
  (bind _outactors (Collision|SphereOverlapActors (Transformation|GetActorLocation) (Variables|Constants|GetSensingRange) (Utilities|Array|MakeArray "ObjectTypeQuery3") "/Script/Engine.Actor"))
  (for _array_element _outactors
    (bind _asbp_master_monster (Utilities|Casting|CastToBP_MasterMonster _array_element))
    (bind _output_get (LocalVariables|SetCurrentTarget%28Local%29 _asbp_master_monster))
    (bind _output_get_2 (LocalVariables|SetCurrentDistance%28Local%29 (Transformation|GetDistanceTo _output_get self)))
    (if (or (< _output_get_2 (LocalVariables|GetBestDistance%28Local%29)) (not (Utilities|IsValid (LocalVariables|GetBestTarget%28Local%29))))
      (bind _result (CallFunction|HasLineOfSight (Transformation|GetWorldLocation (Variables|Default|GetTurretTop)) (Transformation|GetActorLocation (LocalVariables|GetCurrentTarget%28Local%29)) (Utilities|Array|MakeArray self (LocalVariables|GetCurrentTarget%28Local%29))))
      (if _result
        (LocalVariables|SetBestTarget%28Local%29 (LocalVariables|GetCurrentTarget%28Local%29))
        (LocalVariables|SetBestDistance%28Local%29 (LocalVariables|GetCurrentDistance%28Local%29)))))
  (Variables|Private|SetTarget (LocalVariables|GetBestTarget%28Local%29)))

(fn UpdateTurretRotation
  (params (DeltaSeconds :type Float%20%28double-precision%29))
  (Transformation|SetWorldRotation (Variables|Default|GetTurretTop) (Class|KismetMathLibrary|RInterptoConstant (Transformation|GetWorldRotation (Variables|Default|GetTurretTop)) (Math|Rotator|FindLookatRotation (Transformation|GetWorldLocation (Variables|Default|GetTurretTop)) (Transformation|GetActorLocation (Variables|Private|GetTarget))) DeltaSeconds (Variables|Constants|GetRotationSpeed)) false false))

(fn UpdateFire
  (if (> (- (Utilities|Time|GetGameTimeinSeconds) (Variables|Private|GetTimeOfLastFire)) (Variables|Constants|GetRateOfFire))
    (if (> (Math|Vector|DotProduct (Math|Vector|GetUnitDirection(Vector) (Transformation|GetWorldLocation (Variables|Default|GetTurretTop)) (Transformation|GetActorLocation (Variables|Private|GetTarget))) (Math|Vector|GetForwardVector (Variables|Default|GetTurretTop))) 0.99)
      (CallFunction|Fire))))