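; BP_FlameTurret is a turret construct that sweeps back and forth and triggers a fire skill on contact.
; Each Tick, a step counter drives one-degree yaw steps of the root, forward then back over a 120-degree arc, so speed depends on frame rate.
; When an actor overlaps the Box, it prints "Fire" and calls UseSkill for "Fireskill" on that actor's own SkillComponent, targeting that same actor.
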(event OnComponentBeginOverlap(Box)
  (params (OverlappedComponent :type Primitive%20Component%20Object%20Reference) (OtherActor :type Actor%20Object%20Reference) (OtherComp :type Primitive%20Component%20Object%20Reference) (OtherBodyIndex :type Integer) (bFromSweep :type Boolean) (SweepResult :type Hit%20Result%20Structure%20%28by%20ref%29))
  (bind _returnvalue (Actor|GetComponentbyClass OtherActor "/Game/ShootingGame/Blueprints/SkillComponent.SkillComponent_C"))
  (Development|PrintString "Fire")
  (Utilities|IsValid _returnvalue
    (:Is%20Valid
      (Default|UseSkill _returnvalue "Fireskill" OtherActor))))

(event EventBeginPlay)

(event EventTick
  (params (DeltaSeconds :type Float%20%28single-precision%29))
  (if (< (Variables|Default|GetZrotation) 1.2e+02)
    (bind _rotation (CallFunction|Z+Rotation))
    (Variables|Default|SetZrotation _rotation)
    (else
      (bind __rotation (CallFunction|Z-Rotation))
      (bind _output_get (Variables|Default|SetZrotation __rotation))
      (if (== _output_get 2.4e+02)
        (Variables|Default|SetZrotation 0.0)))))

(fn ConstructionScript)

(fn Z+Rotation
  (Transformation|AddWorldRotation (Variables|Default|GetDefaultSceneRoot) (Math|Rotator|MakeRotator 0.0 0.0 1.0) false false)
  (bind _result (Math|Float|IncrementFloat (Variables|Default|GetZrotation))
    (:%20%20
      (return _result))))

(fn Z-Rotation
  (Transformation|AddWorldRotation (Variables|Default|GetDefaultSceneRoot) (Math|Rotator|MakeRotator 0.0 0.0 -1.0) false false)
  (bind _result (Math|Float|IncrementFloat (Variables|Default|GetZrotation))
    (:%20%20
      (return _result))))