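; Minimap controller actor that creates the WG_MiniMap widget on BeginPlay and adds it to the viewport.
; Each tick it writes the player's location and yaw, wrapped and normalized to 0-1, into the MPC_Minimap material parameter collection.
; UpdateIconPosition converts a position's Y into a horizontal icon location on the widget using a hard-coded scale and offset, with vertical fixed at zero.
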(event EventBeginPlay
  (bind _returnvalue (UserInterface|CreateWidget "/Game/LJJ/Minimaps/WG_MiniMap.WG_MiniMap_C"))
  (UserInterface|Viewport|AddtoViewport _returnvalue 0)
  (Variables|Default|Setwdg%20minimap _returnvalue))

(event Collision|EventActorBeginOverlap
  (params (OtherActor :type Actor%20Object%20Reference)))

(event EventTick
  (params (DeltaSeconds :type Float%20%28single-precision%29))
  (bind _returnvalue (Game|GetPlayerCharacter 0))
  (bind _returnvalue_2 (Transformation|GetActorRotation _returnvalue))
  (bind _yaw (Math|Rotator|BreakRotator _returnvalue_2))
  (Rendering|Material|SetVectorParameterValue "/Game/LJJ/Minimaps/MPC_Minimap.MPC_Minimap" "Player" (Math|Conversions|ToLinearColor(Vector) (Transformation|GetActorLocation _returnvalue)) :!class /Script/Engine.KismetMaterialLibrary)
  (Rendering|Material|SetScalarParameterValue "/Game/LJJ/Minimaps/MPC_Minimap.MPC_Minimap" "Player Yaw" (/ (Math|Float|SelectFloat (+ 3.6e+02 _yaw) _yaw (< _yaw 0.0)) 3.6e+02) :!class /Script/Engine.KismetMaterialLibrary))

(event EventUpdateIconPosition
  (params (Position :type Vector%202D%20Structure))
  (Default|UpdateIconLocation (Variables|Default|Getwdg%20minimap) (Math|Vector2D|MakeVector2D (+ (* (.Y (Math|Vector2D|BreakVector2D Position)) 0.35) 7.2e+02) 0.0)))

(fn ConstructionScript)